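; BP_mn_PlayerController is a player controller that registers the game's Enhanced Input contexts and toggles the main menu.
; On BeginPlay it adds the move, camera, UI and swap mapping contexts to the local player subsystem.
; The menu input action creates or removes the main menu widget, switching input mode, mouse cursor and game pause to match.
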(event `self.ReceiveBeginPlay`
  (bind _returnvalue (pcsubsystem `EnhancedInputLocalPlayerSubsystem` self))
  (`/Engine/EditorBlueprintResources/StandardMacros.IsValid` _returnvalue
    (:`Is Valid`
      (`EnhancedInputSubsystemInterface.AddMappingContext` _returnvalue "/Game/_main_mn/input/Input_Move/IMC_mn_Move.IMC_mn_Move" 0 (struct))
      (`EnhancedInputSubsystemInterface.AddMappingContext` _returnvalue "/Game/_main_mn/input/Input_Camera/IMC_mn_Camera.IMC_mn_Camera" 0 (struct))
      (`EnhancedInputSubsystemInterface.AddMappingContext` _returnvalue "/Game/_main_mn/input/Input_UI/IMC_mn_UI.IMC_mn_UI" 0 (struct))
      (`EnhancedInputSubsystemInterface.AddMappingContext` _returnvalue "/Game/_main_mn/input/Input_Swap/IMC_mn_Swap.IMC_mn_Swap" 0 (struct)))))

(event `EnhancedInput|/Game/_main_mn/input/Input_UI/IA_mn_UI_MainMenu`
  (params (ActionValue :type Boolean) (ElapsedSeconds :type "Float (double-precision)") (TriggeredSeconds :type "Float (double-precision)") (InputAction :type "InputAction Object Reference" :default "/Game/_main_mn/input/Input_UI/IA_mn_UI_MainMenu.IA_mn_UI_MainMenu"))
  (:`Triggered`
    (`/Engine/EditorBlueprintResources/StandardMacros.IsValid` (`self.W_MainMenu`)
      (:`Is Valid`
        (`self.Menu_closeUp`))
      (:`Is Not Valid`
        (`self.Menu_openUp`)))))

(fn `Menu_closeUp`
  (`Widget.RemoveFromParent` (`self.W_MainMenu`))
  (set `self.W_MainMenu` null)
  (`WidgetBlueprintLibrary.SetInputMode_GameOnly` self)
  (set `self.bShowMouseCursor` false)
  (`GameplayStatics.SetGamePaused` false))

(fn `Menu_openUp`
  (bind _returnvalue (`|CreateWidget` "/Game/_main_mn/UI/WBP_mn_MainMenu.WBP_mn_MainMenu_C" self))
  (bind _output_get (set `self.W_MainMenu` _returnvalue))
  (`UserWidget.AddToViewport` _output_get 0)
  (`WidgetBlueprintLibrary.SetInputMode_GameAndUIEx` self null)
  (set `self.bShowMouseCursor` true)
  (`GameplayStatics.SetGamePaused` true))

(fn `UserConstructionScript`)