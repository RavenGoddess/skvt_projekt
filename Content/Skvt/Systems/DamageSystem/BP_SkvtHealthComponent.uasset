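; BP_SkvtHealthComponent is a health component in the Skvt damage system that tracks health and signals death.
; DealDamage subtracts damage from Health, clamps the result between zero and MaxHealth, and calls OnDeath whenever the result is zero, including on repeated hits.
; IsDead reports whether Health is zero.
; The component has no active BeginPlay or Tick logic.
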(fn `DealDamage`
  (params (Damage :type "Float (double-precision)"))
  (bind _output_get (set `self.Health` (`KismetMathLibrary.FClamp` (- (`self.Health`) Damage) 0.0 (`self.MaxHealth`))))
  (if (== _output_get 0.0)
    (`self.OnDeath`)))

(fn `IsDead`
  (returns (Dead :type Boolean))
  (return (== (`self.Health`) 0.0)))