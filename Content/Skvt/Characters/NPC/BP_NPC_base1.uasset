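; Base NPC character that takes damage, can be stealth-killed by the player, and ragdolls on death before being destroyed.
; Damage feeds HealthComponent, whose death signal triggers the ragdoll and a timed destroy.
; TakedownArea overlaps toggle the player's CanTakeDown flag and an assassination prompt, rotated each tick against the player controller.
; OnStealthKilled plays a neck-break montage, starts the delayed death and returns a reference transform for positioning the assassin.
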(event `self.HealthComponent.SignalCharDeath`
  (`self.TriggerCharDeath`))

(event `self.ReceiveAnyDamage`
  (params (Damage :type "Float (single-precision)") (DamageType :type "DamageType Object Reference") (InstigatedBy :type "Controller Object Reference") (DamageCauser :type "Actor Object Reference"))
  ;[1 1 1 1 50] Damage system
  (`/Game/Skvt/Systems/HealthComponent.ProcessDamage` (`self.HealthComponent`) Damage)
  (`self.PlayAnimMontage` "/Game/Skvt/Characters/Animations/Attacks/AM_Hit_punch.AM_Hit_punch"))

(event `AssDeath`
  (`CharacterMovementComponent.DisableMovement` (`self.CharacterMovement`))
  (`PrimitiveComponent.SetCollisionResponseToChannel` (`self.CapsuleComponent`) "ECC_Pawn" "ECR_Ignore")
  (`PrimitiveComponent.SetCollisionResponseToChannel` (`self.CapsuleComponent`) "ECC_Camera" "ECR_Ignore")
  (`self.SetActorEnableCollision` true)
  (bind _returnvalue (`self.PlayAnimMontage` "/Game/Skvt/Characters/Animations/Attacks/Hit_BreakNeck_Montage.Hit_BreakNeck_Montage"))
  (`KismetSystemLibrary.Delay` _returnvalue)
  (`self.TriggerCharDeath`))

(event `self.TakedownArea.OnComponentBeginOverlap`
  (params (OverlappedComponent :type "PrimitiveComponent Object Reference") (OtherActor :type "Actor Object Reference") (OtherComp :type "PrimitiveComponent Object Reference") (OtherBodyIndex :type Integer) (bFromSweep :type Boolean) (SweepResult :type "HitResult Structure (by ref)"))
  (if (not (`self.PawnDead`))
    (bind _asbp_skvt_base_char (cast `/Game/Skvt/Characters/BP_SkvtBaseChar` OtherActor))
    (set `/Game/Skvt/Characters/BP_SkvtBaseChar.CanTakeDown?` true _asbp_skvt_base_char)
    (`SceneComponent.SetVisibility` (`self.AssassinationWidget`) true false)))

(event `self.TakedownArea.OnComponentEndOverlap`
  (params (OverlappedComponent :type "PrimitiveComponent Object Reference") (OtherActor :type "Actor Object Reference") (OtherComp :type "PrimitiveComponent Object Reference") (OtherBodyIndex :type Integer))
  (if (not (`self.PawnDead`))
    (bind _asbp_skvt_base_char (cast `/Game/Skvt/Characters/BP_SkvtBaseChar` OtherActor))
    (set `/Game/Skvt/Characters/BP_SkvtBaseChar.CanTakeDown?` false _asbp_skvt_base_char)
    (`SceneComponent.SetVisibility` (`self.AssassinationWidget`) false false)))

(event `self.ReceiveTick`
  (params (DeltaSeconds :type "Float (single-precision)"))
  (if (not (`self.PawnDead`))
    (`SceneComponent.K2_SetWorldRotation` (`self.AssassinationWidget`) (.rotation (`self.GetTransform` (`GameplayStatics.GetPlayerController` 0))) false false)
    (`SceneComponent.K2_AddLocalRotation` (`self.AssassinationWidget`) (struct :`Yaw` 180.0) false false)))

(fn `FinalizeCharDeath`
  (`self.K2_DestroyActor`))

(fn `IsDead`
  (returns (IsDead :type Boolean))
  (return (`/Game/Skvt/Systems/HealthComponent.IsDead` (`self.HealthComponent`))))

(fn `OnStealthKilled`
  (returns (`REF location` :type "Vector Structure") (Rotation :type "Rotator Structure"))
  (bind _ref_pose_assassin (`self.REF POSE ASSASSIN`))
  (set `self.PawnDead` true)
  (`CharacterMovementComponent.DisableMovement` (`self.CharacterMovement`))
  (`PrimitiveComponent.SetCollisionResponseToChannel` (`self.CapsuleComponent`) "ECC_Pawn" "ECR_Ignore")
  (`self.PlayAnimMontage` "/Game/Skvt/Characters/Animations/Attacks/Hit_BreakNeck_Montage.Hit_BreakNeck_Montage")
  (`SceneComponent.SetVisibility` (`self.AssassinationWidget`) false false)
  (`self.AssDeath`)
  (return (`SceneComponent.K2_GetComponentLocation` _ref_pose_assassin) (`SceneComponent.K2_GetComponentRotation` _ref_pose_assassin)))

(fn `TriggerCharDeath`
  (`PrimitiveComponent.SetSimulatePhysics` (`self.Mesh`) true)
  (`CharacterMovementComponent.DisableMovement` (`self.CharacterMovement`))
  (`ActorComponent.K2_DestroyComponent` (`self.CapsuleComponent`))
  (`KismetSystemLibrary.K2_SetTimer` null "FinalizeCharDeath" 5.0))

(fn `TriggerCharDeath_1`
  (`PrimitiveComponent.SetSimulatePhysics` (`self.Mesh`) true)
  (`CharacterMovementComponent.DisableMovement` (`self.CharacterMovement`))
  (`KismetSystemLibrary.K2_SetTimer` null "FinalizeCharDeath" 5.0))

(fn `UserConstructionScript`)