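; BP_Switch2 is an interactable switch actor that turns a set of referenced electric actors on or off.
; Its Interact event loops over ActorsRef and sends ToggleOnMessage with the matching state.
; Only the on path first checks each actor for the BPI_Eletric interface.
; A Box overlap shows the widget on begin and hides it on end, with no filter on the overlapping actor.
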(event `self.ReceiveActorBeginOverlap`
  (params (OtherActor :type "Actor Object Reference")))

(event `/Game/Skvt/Blueprints/BPI_Eletric.Interact`
  (params (Interact :type Boolean))
  (if Interact
    (for _array_element (`self.ActorsRef`)
      (if (`KismetSystemLibrary.DoesImplementInterface` _array_element "/Game/Skvt/Blueprints/BPI_Eletric.BPI_Eletric_C")
        (message `/Game/Skvt/Blueprints/BPI_Eletric.ToggleOn` _array_element true)))
    (else
      (for _array_element_2 (`self.ActorsRef`)
        (message `/Game/Skvt/Blueprints/BPI_Eletric.ToggleOn` _array_element_2 false)))))

(event `self.Box.OnComponentBeginOverlap`
  (params (OverlappedComponent :type "PrimitiveComponent Object Reference") (OtherActor :type "Actor Object Reference") (OtherComp :type "PrimitiveComponent Object Reference") (OtherBodyIndex :type Integer) (bFromSweep :type Boolean) (SweepResult :type "HitResult Structure (by ref)"))
  ;[1 1 1] Visualision Widget
  (`SceneComponent.SetVisibility` (`self.Widget`) true false))

(event `self.Box.OnComponentEndOverlap`
  (params (OverlappedComponent :type "PrimitiveComponent Object Reference") (OtherActor :type "Actor Object Reference") (OtherComp :type "PrimitiveComponent Object Reference") (OtherBodyIndex :type Integer))
  ;[1 1 1] Visualision Widget
  (`SceneComponent.SetVisibility` (`self.Widget`) false false))

(fn `UserConstructionScript`)