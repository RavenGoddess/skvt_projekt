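; BP_TogglePlatform is a platform actor that changes the color of its linked lights when another actor overlaps it.
; ChangeColor loops over the Lights array and calls ChangeLightColor on each element.
; ToggleLights switches those lights on or off, and ToggleOn sends turn-on or turn-off messages to the Electric array.
; Both toggle functions are left unwired in the event graph, and ending the overlap does nothing.
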(event `self.ReceiveActorBeginOverlap`
  (params (OtherActor :type "Actor Object Reference"))
  (`self.ChangeColor`))

(event `self.ReceiveActorEndOverlap`
  (params (OtherActor :type "Actor Object Reference")))

(fn `ChangeColor`
  (for _array_element (`self.Lights`)
    (`/Game/Skvt/Blueprints/Light/BP_WallSconce.ChangeLightColor` _array_element)))

(fn `ToggleLights`
  (params (TurnOn :type Boolean))
  (for _array_element (`self.Lights`)
    (`/Game/Skvt/Blueprints/Light/BP_WallSconce.ToggleLight` _array_element TurnOn)))

(fn `ToggleOn`
  (params (IsOn :type Boolean))
  (for _array_element (`self.Electric`)
    (if IsOn
      (message `/Game/Skvt/Blueprints/BPI_Electric.TurnOn` _array_element)
      (else
        (message `/Game/Skvt/Blueprints/BPI_Electric.TurnOff` _array_element)))))

(fn `UserConstructionScript`)