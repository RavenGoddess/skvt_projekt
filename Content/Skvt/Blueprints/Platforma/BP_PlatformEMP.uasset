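; EMP platform that fires a pulse when anything begins overlapping its Box, disabling nearby electric actors.
; The overlap restarts the SphereMagnification timeline, which draws an expanding blue debug sphere as the pulse visual.
; Every timeline update also adds an audio component and sends DisableByEMPMessage to BPI_Eletric actors inside the Sphere component.
; The affected area is the Sphere component's own overlap volume, independent of the drawn radius.
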(event `self.Box.OnComponentBeginOverlap`
  (params (OverlappedComponent :type "PrimitiveComponent Object Reference") (OtherActor :type "Actor Object Reference") (OtherComp :type "PrimitiveComponent Object Reference") (OtherBodyIndex :type Integer) (bFromSweep :type Boolean) (SweepResult :type "HitResult Structure (by ref)"))
  (bind (_direction _spheremagnification) (`Timeline|SphereMagnification` :`NewTime` (`SphereComponent.GetScaledSphereRadius` (`self.Sphere`)) :!via `PlayFromStart`)
    (:`Update`
      (`KismetSystemLibrary.DrawDebugSphere` (`PrimitiveComponent.GetCenterOfMass` (`self.Sphere`) "None") _spheremagnification 50 (struct :`G` 0.395329 :`B` 1.0 :`A` 1.0) 0.05 1.0)
      (`AddComponent|NODE_AddAudioComponent-1`)
      (for _array_element (`PrimitiveComponent.GetOverlappingActors` (`self.Sphere`) "/Script/Engine.Actor")
        (if (`KismetSystemLibrary.DoesImplementInterface` _array_element "/Game/Skvt/Blueprints/BPI_Eletric.BPI_Eletric_C")
          (message `/Game/Skvt/Blueprints/BPI_Eletric.DisableByEMP` _array_element true))))))

(fn `UserConstructionScript`)