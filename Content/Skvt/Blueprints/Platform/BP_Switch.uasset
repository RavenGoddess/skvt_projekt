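; BP_Switch is an overlap-driven switch that powers a set of electric devices while an actor is on it.
; Begin overlap sends ToggleOnMessage(true) to each entry in the ElectricDevices array, and end overlap sends false.
; It does not filter overlapping actors or count them, so any single exit switches every device off.
; Older loops calling ToggleOnInternal on a Lights array remain disconnected and never run.
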(event `self.ReceiveActorBeginOverlap`
  (params (OtherActor :type "Actor Object Reference"))
  (for _array_element (`self.ElectricDevices`)
    (message `/Game/Skvt/Blueprints/BPI_Electric.ToggleOn` _array_element true)))

(event `self.ReceiveActorEndOverlap`
  (params (OtherActor :type "Actor Object Reference"))
  (for _array_element (`self.ElectricDevices`)
    (message `/Game/Skvt/Blueprints/BPI_Electric.ToggleOn` _array_element false)))

(fn `UserConstructionScript`)