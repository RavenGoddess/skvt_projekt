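; BP_Platform is a trigger platform that switches linked objects while something overlaps its Box component.
; Begin overlap calls ToggleMessage(true) on every element of the Electric array, and end overlap sends false, with no filtering of the overlapping actor.
; Similar loops that call ToggleOn on a Lampy array are disconnected and never run.
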(event `self.Box.OnComponentBeginOverlap`
  (params (OverlappedComponent :type "PrimitiveComponent Object Reference") (OtherActor :type "Actor Object Reference") (OtherComp :type "PrimitiveComponent Object Reference") (OtherBodyIndex :type Integer) (bFromSweep :type Boolean) (SweepResult :type "HitResult Structure (by ref)"))
  (for _array_element (`self.Electric`)
    (message `/Game/Skvt/Blueprints/BPI_Electric.Toggle` _array_element true)))

(event `self.Box.OnComponentEndOverlap`
  (params (OverlappedComponent :type "PrimitiveComponent Object Reference") (OtherActor :type "Actor Object Reference") (OtherComp :type "PrimitiveComponent Object Reference") (OtherBodyIndex :type Integer))
  ;[0.15 0.05165 0.137 0.5] Comment
  (for _array_element (`self.Electric`)
    (message `/Game/Skvt/Blueprints/BPI_Electric.Toggle` _array_element false)))

(fn `UserConstructionScript`)