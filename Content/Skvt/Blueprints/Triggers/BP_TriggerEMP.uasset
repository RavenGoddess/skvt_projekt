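; BP_TriggerEMP is a trigger that fires an EMP blast at nearby electrical devices whenever an actor begins overlapping it.
; The blast function gathers every BP_ElectricalDevices actor, child Blueprints included, and calls EMPBlastMessage on those within a hardcoded radius of the trigger.
; Each hit also draws a long-lived debug sphere showing the blast radius.
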(event `self.ReceiveActorBeginOverlap`
  (params (OtherActor :type "Actor Object Reference"))
  ;[1 1 1] Find All actors within range and Blast them - valid for parent blueprint - Electrical devices
  (`self.EMPBlastAllActorsWithinDistance`))

(fn `EMPBlastAllActorsWithinDistance`
  (bind _returnvalue (`self.K2_GetActorLocation`))
  (bind _outactors (`GameplayStatics.GetAllActorsOfClass` "/Game/Skvt/Blueprints/BP_ElectricalDevices.BP_ElectricalDevices_C"))
  (for _array_element _outactors
    (if (<= (`KismetMathLibrary.VSize` (- (`self.K2_GetActorLocation` _array_element) _returnvalue)) 2000.0)
      (message `/Game/Skvt/Blueprints/BPI01_ElectricDevices.EMP Blast` _array_element)
      (`KismetSystemLibrary.DrawDebugSphere` _returnvalue 2000.0 24 (struct :`R` 1.0 :`G` 1.0 :`B` 1.0 :`A` 1.0) 100.0 10.0))))

(fn `UserConstructionScript`)