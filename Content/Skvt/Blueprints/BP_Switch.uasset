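; BP_Switch is an overlap-triggered switch that changes the color of the lights in its Lamps array.
; Any actor overlap calls SetLightCOlor, which calls ChangeColor on each lamp.
; A ToggleLights function passes IsOn to each lamp's ToggleOnInternal, then flips the flag, but its calls in the event graph, including a Player-tag-gated one, are disconnected.
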(event `self.ReceiveBeginPlay`)

(event `self.ReceiveActorBeginOverlap`
  (params (OtherActor :type "Actor Object Reference"))
  (`self.SetLightCOlor`))

(fn `SetLightCOlor`
  (for _array_element (`self.Lamps`)
    (`/Game/Skvt/Blueprints/Light/BP_WallSconce.ChangeColor` _array_element)))

(fn `ToggleLights`
  (for _array_element (`self.Lamps`)
    (`/Game/Skvt/Blueprints/Light/BP_WallSconce.ToggleOnInternal` _array_element (`self.IsOn`)))
  (set `self.IsOn` (not (`self.IsOn`))))

(fn `UserConstructionScript`)